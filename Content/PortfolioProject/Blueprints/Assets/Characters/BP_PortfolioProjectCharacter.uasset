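; Player character Blueprint that handles key input for pausing and for placing a teleport beam.
; Tab clears all widgets, pauses the game, opens the pause menu and shows the mouse cursor.
; Z plays a sound and spawns a teleport beam at the capsule's transform, destroying the previous one through a stored reference and spawned flag.
; X only plays an eject sound here.
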(event EventBeginPlay)

(event Collision|EventActorBeginOverlap
  (params (OtherActor :type Actor%20Object%20Reference)))

(event EventTick
  (params (DeltaSeconds :type Float%20%28single-precision%29)))

(event Input|KeyboardEvents|Z
  (params (Key :type Key%20Structure))
  (:Pressed
    (Audio|PlaySound2D "/Engine/VREditor/Sounds/UI/Enter_Simulate.Enter_Simulate" 1.0 1.0 0.0 0 0)
    (if (Variables|Default|GetIsSpawned)
      (Actor|DestroyActor (stale _returnvalue)))
    (bind _returnvalue (Game|SpawnActorfromClass "/Game/PortfolioProject/Blueprints/Assets/Actors/BP_PortfolioProjectTeleportBeam.BP_PortfolioProjectTeleportBeam_C" (Transformation|GetWorldTransform (Variables|Default|GetCapsuleComponent)) "AlwaysSpawn" 0 0))
    (Variables|Default|SetIsSpawned true)))

(event Input|KeyboardEvents|Tab
  (params (Key :type Key%20Structure))
  (:Pressed
    (Viewport|RemoveAllWidgets)
    (Game|SetGamePaused true)
    (bind _returnvalue (UserInterface|CreateWidget "/Game/PortfolioProject/Blueprints/Widget/BP_PauseMenu.BP_PauseMenu_C"))
    (UserInterface|Viewport|AddtoViewport _returnvalue 0)
    (Variables|/Script/Engine.PlayerController|SetbShowMouseCursor (Game|GetPlayerController 0) true)))

(event Input|KeyboardEvents|X
  (params (Key :type Key%20Structure))
  (:Pressed
    (Audio|PlaySound2D "/Engine/EditorSounds/GamePreview/EjectFromPlayer.EjectFromPlayer" 1.0 1.0 0.0 0 0)))

(fn ConstructionScript)