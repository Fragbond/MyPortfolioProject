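; Timed ground trigger that opens linked doors when the player character or a pickup actor steps onto it.
; Begin overlap plays a switch sound, then hides each actor in Doors and disables its collision.
; End overlap, unfiltered by actor, replays the sound and restores doors after a five-second Delay.
; That Delay sits inside the loop, so with several doors only the last is restored.
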(event EventBeginPlay)

(event Collision|EventActorBeginOverlap
  (params (OtherActor :type Actor%20Object%20Reference))
  (if (== OtherActor (Game|GetPlayerCharacter 0))
    (Audio|PlaySoundatLocation "/Engine/VREditor/Sounds/UI/Flashlight_Switch.Flashlight_Switch" (Variables|Default|GetGroundTriggerVector) "0, 0, 0" 1.0 1.0 0.0 0 0 0 0 :!label _label)
    (for _array_element (Variables|Default|GetDoors)
      (Rendering|SetActorHiddenInGame _array_element true)
      (Collision|SetActorEnableCollision _array_element false))
    (else
      (bind _asbp_my_portfolio_project_pickup_actor (Utilities|Casting|CastToBP_MyPortfolioProjectPickupActor OtherActor))
      (if (== _asbp_my_portfolio_project_pickup_actor OtherActor)
        (goto _label)))))

(event EventTick
  (params (DeltaSeconds :type Float%20%28single-precision%29)))

(event Collision|EventActorEndOverlap
  (params (OtherActor :type Actor%20Object%20Reference))
  (Audio|PlaySoundatLocation "/Engine/VREditor/Sounds/UI/Flashlight_Switch.Flashlight_Switch" (Variables|Default|GetGroundTriggerVector) "0, 0, 0" 1.0 1.0 0.0 0 0 0 0)
  (for _array_element (Variables|Default|GetDoors)
    (Utilities|FlowControl|Delay 5.0)
    (Rendering|SetActorHiddenInGame _array_element false)
    (Collision|SetActorEnableCollision _array_element true)))

(fn ConstructionScript)